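; BP_PlayerLift is a lift that carries a cube along a spline when the player character (MoronavirusCharacter) enters its trigger box.
; Overlap plays a timeline from the start, and end overlap reverses it from its current position.
; Each timeline update scales the track value by spline length to set the cube's local location and rotation along the spline, keeping its scale, without sweeping.
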(event `self.Box.OnComponentBeginOverlap`
  (params (OverlappedComponent :type "PrimitiveComponent Object Reference") (OtherActor :type "Actor Object Reference") (OtherComp :type "PrimitiveComponent Object Reference") (OtherBodyIndex :type Integer) (bFromSweep :type Boolean) (SweepResult :type "HitResult Structure (by ref)"))
  (bind _spline (`self.Spline`))
  (bind _cube (`self.Cube`))
  (cast `MoronavirusCharacter` OtherActor)
  (bind (_direction _newtrack_0) (`Timeline|Timeline_0` :!via `PlayFromStart` :!label _label)
    (:`Update`
      (bind _returnvalue (* _newtrack_0 (`SplineComponent.GetSplineLength` _spline)))
      (`SceneComponent.K2_SetRelativeTransform` _cube (`KismetMathLibrary.MakeTransform` (`SplineComponent.GetLocationAtDistanceAlongSpline` _spline _returnvalue "Local") (`SplineComponent.GetRotationAtDistanceAlongSpline` _spline _returnvalue "Local") (`SceneComponent.RelativeScale3D` _cube)) false false))))

(event `self.Box.OnComponentEndOverlap`
  (params (OverlappedComponent :type "PrimitiveComponent Object Reference") (OtherActor :type "Actor Object Reference") (OtherComp :type "PrimitiveComponent Object Reference") (OtherBodyIndex :type Integer))
  (cast `MoronavirusCharacter` OtherActor)
  (goto _label :!via `Reverse`))

(fn `UserConstructionScript`)