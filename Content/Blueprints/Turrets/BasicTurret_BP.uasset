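; BasicTurret_BP is a turret actor with a world-space ammo widget.
; On BeginPlay it casts the widget component's user widget to Turret_Ammo_Widget_BP and hands it a reference to itself.
; Each tick it rotates the widget toward the first player's controlled pawn, billboard style, while that pawn is valid.
; The graph contains no targeting or firing logic, and the construction script is empty.
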(event `self.ReceiveBeginPlay`
  (bind _asturret_ammo_widget_bp (cast `/Game/Blueprints/UI/Widgets/Turret_Ammo_Widget_BP` (`WidgetComponent.GetWidget` (`self.Widget`))))
  (set `/Game/Blueprints/UI/Widgets/Turret_Ammo_Widget_BP.Turret` self _asturret_ammo_widget_bp))

(event `self.ReceiveTick`
  (params (DeltaSeconds :type "Float (single-precision)"))
  (bind _widget (`self.Widget`))
  (bind _returnvalue (`Controller.K2_GetPawn` (`GameplayStatics.GetPlayerController` 0)))
  (`/Engine/EditorBlueprintResources/StandardMacros.IsValid` _returnvalue
    (:`Is Valid`
      (`SceneComponent.K2_SetWorldRotation` _widget (`KismetMathLibrary.FindLookAtRotation` (`SceneComponent.K2_GetComponentLocation` _widget) (`self.K2_GetActorLocation` _returnvalue)) false false))))

(fn `UserConstructionScript`)