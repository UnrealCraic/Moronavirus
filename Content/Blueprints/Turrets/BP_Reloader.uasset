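; BP_Reloader is a reload station that refills its linked Turret when the player presses R nearby, then goes on a restock cooldown.
; A sphere overlap flags proximity and shows a widget that turns each tick to face the player's pawn.
; Reloading turns the cylinder red until the restock timer restores it to green.
; A success or failure sound plays on each nearby press.
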(event `self.ReceiveBeginPlay`
  (`self.EnableInput` (`GameplayStatics.GetPlayerController` 0)))

(event `self.ReceiveTick`
  (params (DeltaSeconds :type "Float (single-precision)"))
  (bind _widget (`self.Widget`))
  (bind _returnvalue (`Controller.K2_GetPawn` (`GameplayStatics.GetPlayerController` 0)))
  (`/Engine/EditorBlueprintResources/StandardMacros.IsValid` _returnvalue
    (:`Is Valid`
      (`SceneComponent.K2_SetWorldRotation` _widget (`KismetMathLibrary.FindLookAtRotation` (`SceneComponent.K2_GetComponentLocation` _widget) (`self.K2_GetActorLocation` _returnvalue)) false false))))

(event `self.Sphere.OnComponentBeginOverlap`
  (params (OverlappedComponent :type "PrimitiveComponent Object Reference") (OtherActor :type "Actor Object Reference") (OtherComp :type "PrimitiveComponent Object Reference") (OtherBodyIndex :type Integer) (bFromSweep :type Boolean) (SweepResult :type "HitResult Structure (by ref)"))
  (`SceneComponent.SetVisibility` (`self.Widget`) true false)
  (set `self.PlayerNearby` true))

(event `self.Sphere.OnComponentEndOverlap`
  (params (OverlappedComponent :type "PrimitiveComponent Object Reference") (OtherActor :type "Actor Object Reference") (OtherComp :type "PrimitiveComponent Object Reference") (OtherBodyIndex :type Integer))
  (`SceneComponent.SetVisibility` (`self.Widget`) false false)
  (set `self.PlayerNearby` false))

(event `Key|R`
  (params (Key :type "Key Structure"))
  (bind _playernearby (`self.PlayerNearby`))
  (:`Pressed`
    (if (and _playernearby (`self.CanReload`))
      (`MVTurret.Reload` (`self.Turret`))
      (`KismetSystemLibrary.K2_SetTimerDelegate` (delegate `Restock`) (`self.RestockTime`))
      (`PrimitiveComponent.SetMaterial` (`self.Cylinder`) 0 "/AnimationSharing/AnimSharingRed.AnimSharingRed")
      (`GameplayStatics.PlaySoundAtLocation` "/Engine/EditorSounds/GamePreview/EndSimulate_Cue.EndSimulate_Cue" (`self.K2_GetActorLocation`) (struct) 1.0 1.0 0.0 null null null)
      (set `self.CanReload` false)
      (elif _playernearby
        (`GameplayStatics.PlaySoundAtLocation` "/Engine/EditorSounds/Notifications/CompileFailed_Cue.CompileFailed_Cue" (`self.K2_GetActorLocation`) (struct) 1.0 1.0 0.0 null null null)))))

(event `Restock`
  (`PrimitiveComponent.SetMaterial` (`self.Cylinder`) 0 "/AnimationSharing/AnimSharingGreen.AnimSharingGreen")
  (set `self.CanReload` true))

(fn `UserConstructionScript`)