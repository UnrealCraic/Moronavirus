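; Oxygen tank weapon Blueprint that instantly kills AI characters caught by its hit sphere.
; The Sphere starts with collision off and ignores the tank and its owner when moving.
; ApexStarted enables query-only collision and ApexEnded disables it, limiting hits to that apex window.
; Any AICharacterBase that begins overlapping the Sphere has Kill called on it.
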(event `self.ReceiveBeginPlay`
  (bind _sphere (`self.Sphere`))
  (`PrimitiveComponent.SetCollisionEnabled` _sphere "NoCollision")
  (`PrimitiveComponent.IgnoreActorWhenMoving` _sphere (`self.GetOwner`) true)
  (`PrimitiveComponent.IgnoreActorWhenMoving` _sphere self true))

(event `self.Sphere.OnComponentBeginOverlap`
  (params (OverlappedComponent :type "PrimitiveComponent Object Reference") (OtherActor :type "Actor Object Reference") (OtherComp :type "PrimitiveComponent Object Reference") (OtherBodyIndex :type Integer) (bFromSweep :type Boolean) (SweepResult :type "HitResult Structure (by ref)"))
  (bind _asaicharacter_base (cast `/Game/Blueprints/AI/AICharacterBase` OtherActor))
  (`/Game/Blueprints/AI/AICharacterBase.Kill` _asaicharacter_base))

(fn `ApexEnded`
  (`PrimitiveComponent.SetCollisionEnabled` (`self.Sphere`) "NoCollision"))

(fn `ApexStarted`
  (`PrimitiveComponent.SetCollisionEnabled` (`self.Sphere`) "QueryOnly"))

(fn `UserConstructionScript`)