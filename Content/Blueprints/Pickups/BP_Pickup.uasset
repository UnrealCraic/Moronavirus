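; BP_Pickup is a money pickup that spins in place and expires on its own after a fixed lifespan.
; Tick yaws the actor by a rotation rate variable.
; When a MoronavirusCharacter overlaps its sphere, it adds its value to that character's money, plays a sound at its location and destroys itself.
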(event `self.ReceiveBeginPlay`
  (`self.SetLifeSpan` 30.0))

(event `self.ReceiveTick`
  (params (DeltaSeconds :type "Float (single-precision)"))
  (`self.K2_AddActorWorldRotation` (`KismetMathLibrary.MakeRotator` 0.0 0.0 (* DeltaSeconds (`self.RotationRate`)))))

(event `self.Sphere.OnComponentBeginOverlap`
  (params (OverlappedComponent :type "PrimitiveComponent Object Reference") (OtherActor :type "Actor Object Reference") (OtherComp :type "PrimitiveComponent Object Reference") (OtherBodyIndex :type Integer) (bFromSweep :type Boolean) (SweepResult :type "HitResult Structure (by ref)"))
  (bind _asmoronavirus_character (cast `MoronavirusCharacter` OtherActor))
  (`MoronavirusCharacter.AddMoney` _asmoronavirus_character (`self.Value`))
  (`GameplayStatics.PlaySoundAtLocation` "/Engine/VREditor/Sounds/UI/Laser_Push.Laser_Push" (`self.K2_GetActorLocation`) (struct) 1.0 1.0 0.0 null null null)
  (`self.K2_DestroyActor`))

(fn `UserConstructionScript`)