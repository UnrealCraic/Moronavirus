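; Base AI character that seeks the closest Hospital_BP on BeginPlay and attacks it.
; It moves to a random attack point supplied by the target, retrying after a short delay when blocked.
; Overlapping the target stops movement, turns the character on yaw only, and starts a looping damage timer.
; Death clears the timer, switches the capsule to a dead collision profile, and occasionally spawns a pickup.
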(event `self.ReceiveBeginPlay`
  (bind _newparam (`self.GetClosestTarget`))
  (`/Engine/EditorBlueprintResources/StandardMacros.IsValid` _newparam
    (:`Is Valid`
      (set `self.CurrentTarget` _newparam)
      (`self.MoveToTarget`))))

(event `MoveToTarget`
  (bind _returnvalue (`AIBlueprintHelperLibrary.GetAIController` (`self.GetController`)))
  (bind _returnvalue_2 (`MVHospital.GetRandomAttackTargetFrom` (`self.CurrentTarget`) (`self.K2_GetActorLocation`)))
  (add `AIController.ReceiveMoveCompleted` _returnvalue (delegate `MoveCompleted`))
  (`AIController.MoveToLocation` _returnvalue _returnvalue_2 -1.0 true true false true null true))

(event `MoveCompleted`
  (params (RequestID :type "AIRequestID Structure") (Result :type "EPathFollowingResult Enum" :default "Success"))
  (switch `EPathFollowingResult` Result
    (:`Blocked`
      (`KismetSystemLibrary.Delay` 0.2)
      (`self.MoveToTarget`))))

(event `self.ReceiveActorBeginOverlap`
  (params (OtherActor :type "Actor Object Reference"))
  (bind _currenttarget (`self.CurrentTarget`))
  (if (== OtherActor _currenttarget)
    (`self.StartAttacking` _currenttarget)))

(event `self.Die`
  (`parent.Die`)
  (`self.Kill`))

(fn `DropReward`
  (`|SpawnActorFromClass` (`self.PickupClass`) (`KismetMathLibrary.MakeTransform` (`self.K2_GetActorLocation`)) "Undefined" "OverrideRootScale" null null))

(fn `GetClosestTarget`
  (returns (NewParam :type "MVHospital Object Reference"))
  (locals (CurrentClosestDistance :type "Float (double-precision)" :default 99999997952.0) (ClosestActor :type "MVHospital Object Reference"))
  (bind _outactors (`GameplayStatics.GetAllActorsOfClass` "/Game/Blueprints/Buildings/Hospital/Hospital_BP.Hospital_BP_C"))
  (for _array_element _outactors
    (bind _returnvalue (`self.GetDistanceTo` _array_element self))
    (if (< _returnvalue (`local.CurrentClosestDistance`))
      (set `local.CurrentClosestDistance` _returnvalue)
      (set `local.ClosestActor` _array_element)))
  (return (`local.ClosestActor`)))

(fn `Kill`
  (`KismetSystemLibrary.K2_ClearAndInvalidateTimerHandle` (`self.AttackTimerHandle`))
  (`MovementComponent.StopMovementImmediately` (`self.CharacterMovement`))
  (set `self.IsDead` true)
  (`self.DisableInput` null)
  (`PrimitiveComponent.SetCollisionProfileName` (`self.CapsuleComponent`) "DeadAI" true)
  (`PrimitiveComponent.SetSimulatePhysics` (`self.Mesh`) false)
  (if (< (`KismetMathLibrary.RandomFloatInRange` 0.0 100.0) 10.0)
    (`self.DropReward`)))

(fn `PerformAttack`
  (`GameplayStatics.ApplyDamage` (`self.CurrentTarget`) (`self.Damage`) (`self.GetController`) self "/Script/Engine.DamageType"))

(fn `StartAttacking`
  (params (ActorToAttack :type "Actor Object Reference"))
  (set `self.Attacking` true)
  (`MovementComponent.StopMovementImmediately` (`self.CharacterMovement`))
  (`self.K2_SetActorRotation` (`KismetMathLibrary.MakeRotator` (.roll (`self.K2_GetActorRotation`)) (.pitch (`self.K2_GetActorRotation`)) (.yaw (`KismetMathLibrary.FindLookAtRotation` (`self.K2_GetActorLocation`) (`self.K2_GetActorLocation` ActorToAttack)))))
  (`self.PerformAttack`)
  (bind _returnvalue (`KismetSystemLibrary.K2_SetTimer` null "PerformAttack" (`self.TimeBetweenAttacks`) true))
  (set `self.AttackTimerHandle` _returnvalue))

(fn `UserConstructionScript`)